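; BP_Gun is a weapon actor that agents pick up on touch and that can switch between dropped and equipped states.
; When its Detection volume overlaps a BP_Agent without a valid Primary weapon, it calls that agent's PickupWeapon with itself.
; Drop turns on body physics with a ragdoll collision profile and re-enables detection queries.
; Equip turns off physics, applies the Weapon profile and disables detection.
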(event `self.Detection.OnComponentBeginOverlap`
  (params (OverlappedComponent :type "PrimitiveComponent Object Reference") (OtherActor :type "Actor Object Reference") (OtherComp :type "PrimitiveComponent Object Reference") (OtherBodyIndex :type Integer) (bFromSweep :type Boolean) (SweepResult :type "HitResult Structure (by ref)"))
  (bind _asbp_agent (cast `/Game/Dynamic/Agents/BP_Agent` OtherActor))
  (`KismetSystemLibrary.PrintString` "PickingUp")
  (`/Engine/EditorBlueprintResources/StandardMacros.IsValid` (`/Game/Dynamic/Agents/BP_Agent.Primary` _asbp_agent)
    (:`Is Not Valid`
      (`/Game/Dynamic/Agents/BP_Agent.Pickup_Weapon` _asbp_agent self))))

(event `self.Detection.OnComponentEndOverlap`
  (params (OverlappedComponent :type "PrimitiveComponent Object Reference") (OtherActor :type "Actor Object Reference") (OtherComp :type "PrimitiveComponent Object Reference") (OtherBodyIndex :type Integer))
  (cast `/Game/Dynamic/Agents/BP_Agent` OtherActor))

(fn `Drop`
  (bind _body (`self.Body`))
  (`PrimitiveComponent.SetCollisionProfileName` _body "RagdollWeapon" true)
  (`PrimitiveComponent.SetSimulatePhysics` _body true)
  (`PrimitiveComponent.SetCollisionEnabled` (`self.Detection`) "QueryOnly"))

(fn `Equip`
  (bind _body (`self.Body`))
  (`PrimitiveComponent.SetSimulatePhysics` _body false)
  (`PrimitiveComponent.SetCollisionProfileName` _body "Weapon" true)
  (`PrimitiveComponent.SetCollisionEnabled` (`self.Detection`) "NoCollision"))

(fn `UserConstructionScript`)