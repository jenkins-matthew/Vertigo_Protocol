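; BP_Agent is a first-person character with look, movement, jump, crouch toggle and weapon pickup.
; Timelines shift the camera boom's height for crouching and for dips on jump and landing.
; Leaving the ground starts a speed-scaled coyote timer, cleared on landing, though its callback is empty.
; Weapon pickup stores the weapon as Primary, equips it and snaps its body to WeaponHolder.
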(event `InputAxis|LookUp/Down`
  (params (AxisValue :type "Float (single-precision)"))
  (bind _output_get (set `self.LookupAxisValue` (* AxisValue (`self.LookSensitivity`))))
  (`self.AddControllerPitchInput` _output_get))

(event `InputAxis|LookLeft/Right`
  (params (AxisValue :type "Float (single-precision)"))
  (bind _output_get (set `self.TurnAxisValue` (* AxisValue (`self.LookSensitivity`))))
  (`self.AddControllerYawInput` _output_get))

(event `InputAxis|MoveForward/Backwards`
  (params (AxisValue :type "Float (single-precision)"))
  (bind (_returnvalue_roll _returnvalue_pitch _returnvalue_yaw) (`KismetMathLibrary.BreakRotator` (`self.GetControlRotation`)))
  (bind _output_get (set `self.Forward Axis Value` AxisValue))
  (`self.AddMovementInput` (`KismetMathLibrary.GetForwardVector` (`KismetMathLibrary.MakeRotator` 0.0 0.0 _returnvalue_yaw)) _output_get))

(event `InputAxis|MoveRight/Left`
  (params (AxisValue :type "Float (single-precision)"))
  (bind (_returnvalue_roll _returnvalue_pitch _returnvalue_yaw) (`KismetMathLibrary.BreakRotator` (`self.GetControlRotation`)))
  (bind _output_get (set `self.Right Axis Value` AxisValue))
  (`self.AddMovementInput` (`KismetMathLibrary.GetRightVector` (`KismetMathLibrary.MakeRotator` _returnvalue_roll 0.0 _returnvalue_yaw)) _output_get))

(event `InputAction|JumpAction`
  (params (Key :type "Key Structure"))
  (:`Pressed`
    (if (and (`self.CanJump`) (not (`NavMovementComponent.IsCrouching` (`self.CharacterMovement`))))
      (`self.Jump`)
      (`TimelineComponent.PlayFromStart` (`self.DipCamera`)))))

(event `InputAction|Crouch`
  (params (Key :type "Key Structure"))
  (bind _crouchcamera (`self.CrouchCamera`))
  (bind _charactermovement (`self.CharacterMovement`))
  (:`Pressed`
    (if (not (`NavMovementComponent.IsFalling` _charactermovement))
      (if (not (`NavMovementComponent.IsCrouching` _charactermovement))
        (`self.Crouch`)
        (`TimelineComponent.Play` _crouchcamera)
        (else
          (`self.UnCrouch`)
          (`TimelineComponent.Reverse` _crouchcamera))))))

(event `self.OnLanded`
  (params (Hit :type "HitResult Structure (by ref)"))
  (`KismetSystemLibrary.K2_ClearAndInvalidateTimerHandle` (`self.CoyoteTimer`))
  (`TimelineComponent.PlayFromStart` (`self.DipCamera`)))

(event `self.K2_OnMovementModeChanged`
  (params (PrevMovementMode :type "EMovementMode Enum" :default "MOVE_None") (NewMovementMode :type "EMovementMode Enum" :default "MOVE_None") (PrevCustomMode :type Byte) (NewCustomMode :type Byte))
  (if (`|EnumEquality` NewMovementMode "MOVE_Falling")
    (bind _returnvalue (`KismetSystemLibrary.K2_SetTimerDelegate` (delegate `CoyoteTime`) (* (`KismetMathLibrary.Lerp` 0.25 1.0 (`KismetMathLibrary.FClamp` (`KismetMathLibrary.NormalizeToRange` (`KismetMathLibrary.VSize` (`self.GetVelocity`)) 0.0 (`MovementComponent.GetMaxSpeed` (`self.CharacterMovement`))))) (`self.CoyoteTimer_Time`))))
    (set `self.CoyoteTimer` _returnvalue)))

(event `CoyoteTime`)

(event `Pickup_Weapon`
  (params (Weapon :type "/Game/Dynamic/Weapons/BP_Gun Object Reference"))
  (bind _output_get (set `self.Primary` Weapon))
  (`/Game/Dynamic/Weapons/BP_Gun.Equip` _output_get)
  (`SceneComponent.K2_AttachToComponent` (`/Game/Dynamic/Weapons/BP_Gun.Body` _output_get) (`self.WeaponHolder`) "None" "SnapToTarget" "SnapToTarget" "SnapToTarget" true))

(fn `UserConstructionScript`)